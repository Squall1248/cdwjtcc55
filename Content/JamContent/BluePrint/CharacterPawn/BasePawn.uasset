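; BasePawn is a combat pawn with health that faces the FightCamera like a billboard, yawing every tick.
; Attack moves it via AI to a target, triggers the target's HitShake, then returns it to its BeginPlay location and notifies the widget.
; HitShake plays a timeline pitch wobble, then applies the hit pawn's own AttackDamage to its Health.
; Lethal damage only sets IsDie, which blocks further hit reactions.
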(event `self.ReceiveBeginPlay`
  (bind _returnvalue (`GameplayStatics.GetActorOfClass` "/Game/JamContent/BluePrint/FightBluePrint/FightCamera.FightCamera_C"))
  (set `self.ViewCamera` _returnvalue)
  (set `self.BaseLocation` (`self.K2_GetActorLocation`)))

(event `self.ReceiveTick`
  (params (DeltaSeconds :type "Float (single-precision)"))
  (`self.CamAlign` self (`self.ViewCamera`)))

(event `ReturnBaseLoc`
  (`|AIMoveTo` self (`self.BaseLocation`) null))

(event `Attack`
  (params (TargetActor :type "Actor Object Reference") (Widget :type "/Game/JamContent/BluePrint/WidgetBluePrint/FightWidget Object Reference"))
  (`|AIMoveTo` self (0.0 0.0 0.0) TargetActor 100.0
    (:`OnSuccess`
      (`self.HitShake` (cast `/Game/JamContent/BluePrint/CharacterPawn/BasePawn` TargetActor :!pure true))
      (`KismetSystemLibrary.Delay` 1.0)
      (`self.ReturnBaseLoc`)
      (message `/Game/JamContent/BluePrint/FightBluePrint/FightInterface.EndAttack` Widget))))

(event `HitShake`
  (if (not (`self.IsDie`))
    (bind (_direction _newtrack_1) (`Timeline|Hit` :!via `PlayFromStart`)
      (:`Update`
        (`self.K2_SetActorRelativeRotation` (`KismetMathLibrary.MakeRotator` 0.0 (* _newtrack_1 90.0))))
      (:`Finished`
        (`self.DamageF` (`self.AttackDamage`))))))

(fn `CamAlign`
  (params (Sprite :type "Actor Object Reference") (ViewCam :type "Actor Object Reference"))
  (bind (_returnvalue_roll _returnvalue_pitch) (`KismetMathLibrary.BreakRotator` (`self.K2_GetActorRotation` Sprite)))
  (bind (_returnvalue_x _returnvalue_y) (`KismetMathLibrary.BreakVector` (- (`self.K2_GetActorLocation` Sprite) (`self.K2_GetActorLocation` ViewCam))))
  (bind _outdir (`KismetMathLibrary.ToDirectionAndLength2D` (`KismetMathLibrary.MakeVector2D` _returnvalue_x _returnvalue_y)))
  (`self.K2_SetActorRotation` (`KismetMathLibrary.MakeRotator` _returnvalue_roll _returnvalue_pitch (+ (`KismetMathLibrary.DegAtan2` (`.Y` (`KismetMathLibrary.BreakVector2D` _outdir)) (`KismetMathLibrary.BreakVector2D` _outdir)) 90.0))))

(fn `DamageF`
  (params (Damage :type Integer))
  (bind _returnvalue (- (`self.Health`) Damage))
  (if (> _returnvalue 0)
    (set `self.Health` _returnvalue)
    (`KismetSystemLibrary.PrintString` (`KismetStringLibrary.Conv_IntToString` (`self.Health`)))
    (else
      (`self.Die`))))

(fn `Die`
  (set `self.IsDie` true))

(fn `UserConstructionScript`)