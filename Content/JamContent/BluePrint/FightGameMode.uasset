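; Game mode for the fight level that sets up a battle between the player's saved rats and enemies.
; On BeginPlay it loads the GameSave slot, switches the view to the FightCamera and spawns allies or enemies at each SpawnPoint according to its IsPlayerSpawn flag.
; Non-enemy allies take name and combat stats from saved PlayerRats by a running index.
; Both combatant arrays then feed a newly created FightWidget.
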(event `self.ReceiveBeginPlay`
  (`self.LoadSave`)
  (bind _returnvalue (`GameplayStatics.GetActorOfClass` "/Game/JamContent/BluePrint/FightBluePrint/FightCamera.FightCamera_C"))
  (`PlayerController.SetViewTargetWithBlend` (`GameplayStatics.GetPlayerController` 0) _returnvalue 0.0 "VTBlend_Linear" 0.0 false)
  (`self.SpawnPawn`)
  (bind _returnvalue_2 (`|CreateWidget` "/Game/JamContent/BluePrint/WidgetBluePrint/FightWidget.FightWidget_C" null (`self.ActivePawn`) (`self.ActivePlayer`)))
  (`UserWidget.AddToViewport` _returnvalue_2 0))

(fn `LoadSave`
  (bind _returnvalue (`GameplayStatics.LoadGameFromSlot` "GameSave"))
  (bind _asplayer_save (cast `/Game/JamContent/BluePrint/PlayerSave` _returnvalue))
  (set `self.PlayerSave` _asplayer_save))

(fn `SetRatsPlayer`
  (locals (RatsIndex :type Integer))
  (bind (_name _curenthp _maxhp _initiative _baseattackdamage) (break `/Game/JamContent/BluePrint/DataTypes/RatData` (`|GetArrayItem` (`/Game/JamContent/BluePrint/PlayerSave.PlayerRats` (`self.PlayerSave`)) (`local.RatsIndex`))))
  (`self.LoadSave`)
  (for _array_element (`self.ActivePlayer`)
    (if (not (`/Game/JamContent/BluePrint/CharacterPawn/BasePawn.enemies` _array_element))
      (set `/Game/JamContent/BluePrint/CharacterPawn/BasePawn.Health` _curenthp _array_element)
      (set `/Game/JamContent/BluePrint/CharacterPawn/BasePawn.MaxHealth` _maxhp _array_element)
      (set `/Game/JamContent/BluePrint/CharacterPawn/BasePawn.Initiative` _initiative _array_element)
      (set `/Game/JamContent/BluePrint/CharacterPawn/BasePawn.AttackDamage` _baseattackdamage _array_element)
      (set `/Game/JamContent/BluePrint/CharacterPawn/BasePawn.Name` _name _array_element)
      (`/Engine/EditorBlueprintResources/StandardMacros.IncrementInt` (`local.RatsIndex`)))))

(fn `SpawnPawn`
  (bind _outactors (`GameplayStatics.GetAllActorsOfClass` "/Game/JamContent/BluePrint/FightBluePrint/SpawnPoint.SpawnPoint_C"))
  (for _array_element _outactors
    (if (`/Game/JamContent/BluePrint/FightBluePrint/SpawnPoint.IsPlayerSpawn` _array_element)
      (bind _returnvalue (`|SpawnActorFromClass` "/Game/JamContent/BluePrint/CharacterPawn/AlliedCharacter.AlliedCharacter_C" (`KismetMathLibrary.MakeTransform` (`self.K2_GetActorLocation` _array_element) (`self.K2_GetActorRotation` _array_element)) "AlwaysSpawn" "MultiplyWithRoot" null null))
      (bind _returnvalue_2 (`KismetArrayLibrary.Array_Add` (`self.ActivePlayer`) _returnvalue))
      (`KismetSystemLibrary.PrintString` (`KismetStringLibrary.Conv_IntToString` _returnvalue_2))
      (else
        (bind _returnvalue_3 (`|SpawnActorFromClass` "/Game/JamContent/BluePrint/CharacterPawn/EnemieCharacter.EnemieCharacter_C" (`KismetMathLibrary.MakeTransform` (`self.K2_GetActorLocation` _array_element) (`self.K2_GetActorRotation` _array_element)) "AlwaysSpawn" "MultiplyWithRoot" null null))
        (`KismetArrayLibrary.Array_Add` (`self.ActivePawn`) _returnvalue_3))))
  (`self.SetRatsPlayer`))

(fn `UserConstructionScript`)